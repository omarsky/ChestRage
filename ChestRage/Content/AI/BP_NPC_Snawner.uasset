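; NPC spawner actor that keeps spawning random NPC variants at reachable navmesh points within a radius around itself.
; A looping timer with slight start-delay variance spawns one NPC per tick while the alive count is below the cap.
; Each spawn increments that count and binds its OnDestroyed event to decrement it, so freed slots refill.
; Debug events toggle a timer-driven sphere showing the spawn radius and randomize its color.
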(event Custom|Spawn%20AI
  (bind _returnvalue (Transformation|GetActorLocation))
  (bind _spawn_radius (Variables|Publicvariables|GetSpawn%20Radius))
  (bind (_randomlocation _returnvalue_2) (AI|Navigation|GetRandomReachablePointinRadius _returnvalue _spawn_radius 0 0))
  (if (< (Variables|Default|GetCurrent%20Alive%20Enemies) (Variables|PublicVariables|GetMax%20spawned%20count))
    (if _returnvalue_2
      (bind _returnvalue_3 (Game|SpawnActorfromClass (.OutItem (Utilities|Array|Random (Variables|PublicVariables|GetNPC%20variants))) (Math|Transform|MakeTransform _randomlocation "0, 0, 0" "1.000000,1.000000,1.000000") "Undefined" "MultiplyWithRoot" self 0))
      (Utilities|FlowControl|Sequence
        (:then_0
          (Math|Integer|IncrementInt (Variables|Default|GetCurrent%20Alive%20Enemies)))
        (:then_1
          (Game|BindEventtoOnDestroyed _returnvalue_3 (delegate Custom|NPC%20Killed)))))))

(event Custom|Debug:%20toggle%20debug%20render
  ;[1 0 0 0.5] Debug render
  (bind _output_get (Variables|Debug|SetIs%20Rendering%20Debug (not (Variables|Debug|GetIs%20Rendering%20Debug))))
  (Utilities|Time|SetTimerbyEvent (delegate Custom|Debug:%20show%20radius%20once) (Math|Float|SelectFloat 0.5 0.0 _output_get) true))

(event Custom|Debug:%20show%20radius%20once
  ;[1 0 0 0.5] Debug render
  (Rendering|Debug|DrawDebugSphere (Transformation|GetActorLocation) (Variables|Publicvariables|GetSpawn%20Radius) 20 (Variables|Debug|GetDebug%20color) 0.5))

(event Custom|NPC%20Killed
  (params (DestroyedActor :type Actor%20Object%20Reference))
  (Math|Integer|DecrementInt (Variables|Default|GetCurrent%20Alive%20Enemies)))

(event Custom|Debug:%20random%20color
  ;[1 0 0 0.5] Debug render
  (Class|KismetMathLibrary|LinearColorSetRandomHue (Variables|Debug|GetDebug%20color)))

(event EventBeginPlay
  (bind _spawn_delay (Variables|PublicVariables|GetSpawn%20Delay))
  ;[0.15 0.15 0.15 0.5] Check if we have what to spawn
  (if (Utilities|Array|IsNotEmpty (Variables|PublicVariables|GetNPC%20variants))
    (Utilities|Time|SetTimerbyEvent (delegate Custom|Spawn%20AI) _spawn_delay true false 0.0 (* _spawn_delay 0.1))))

(fn ConstructionScript)