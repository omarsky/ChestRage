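; Ranged NPC Blueprint that fires a projectile when it receives a ShootCommand event with a location and rotation.
; The event spawns BP_FirstPersonProjectile at that location pushed out by a rotated offset, then plays the template weapon fire sound there.
; The spawn logic is copied from the first-person template weapon, and a todo notes the projectile may be replaced.
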(event Custom|Event%20Shoot%20Command
  (params (Location :type Vector) (Rotation :type Rotator))
  (bind _projectileoffset (Variables|Default|GetProjectileOffset))
  (bind _returnvalue (Math|Vector|RotateVector _projectileoffset Rotation))
  (bind _returnvalue_2 (+ Location _returnvalue))
  ;[0.05 0.05 0.05] Projectile Spawn Logic )copied from template weapon)
  (Game|SpawnActorfromClass "/Game/FirstPerson/Blueprints/BP_FirstPersonProjectile.BP_FirstPersonProjectile_C" (Math|Transform|MakeTransform _returnvalue_2 Rotation) "Undefined" "OverrideRootScale" 0 0) ; todo: replace with our projectile?
  (Audio|PlaySoundatLocation "/Game/FPWeapon/Audio/FirstPersonTemplateWeaponFire02.FirstPersonTemplateWeaponFire02" _returnvalue_2 "0, 0, 0" 1.0 1.0 0.0 0 0 0 0) ; Play firing sound
)

(event EventBeginPlay
  (|CallParentFunction) ; This node is disabled and will not be called.\nDrag off pins to build functionality.
)

(event Collision|EventActorBeginOverlap
  (params (OtherActor :type Actor%20Object%20Reference))
  (|CallParentFunction OtherActor) ; This node is disabled and will not be called.\nDrag off pins to build functionality.
)

(event EventTick
  (params (DeltaSeconds :type Float%20%28single-precision%29))
  (|CallParentFunction DeltaSeconds) ; This node is disabled and will not be called.\nDrag off pins to build functionality.
)

(fn ConstructionScript
  (|CallParentFunction))