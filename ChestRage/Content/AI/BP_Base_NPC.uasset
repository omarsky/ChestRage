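; Base NPC character that hurts the first-person player on contact and drops a password note when damaged.
; Hitting the player applies damage, launches the NPC along the hit normal, and sets a DamagedPlayerRecently blackboard flag for its AI.
; Any damage spawns a BP_PasswordNote at the capsule's location and rotation with unit scale, so enemy scaling does not affect it, then destroys the NPC.
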(event EventBeginPlay)

(event Collision|EventActorBeginOverlap
  (params (OtherActor :type Actor%20Object%20Reference)))

(event EventTick
  (params (DeltaSeconds :type Float%20%28single-precision%29)))

(event Collision|EventHit
  (params (MyComp :type Primitive%20Component%20Object%20Reference) (Other :type Actor%20Object%20Reference) (OtherComp :type Primitive%20Component%20Object%20Reference) (bSelfMoved :type Boolean) (HitLocation :type Vector :default "0, 0, 0") (HitNormal :type Vector :default "0, 0, 0") (NormalImpulse :type Vector :default "0, 0, 0") (Hit :type Hit%20Result%20Structure%20%28by%20ref%29))
  (bind _asbp_first_person_character (Utilities|Casting|CastToBP_FirstPersonCharacter Other))
  ;[0.15 0.15 0.15 0.5] Apply damage
  (Game|Damage|ApplyDamage _asbp_first_person_character 1.0 0 self)
  (Character|LaunchCharacter (* HitNormal (Variables|Default|GetPush%20from%20collision%20force)) false false)
  (AI|Components|Blackboard|SetValueasBool (AI|GetBlackboard 0) (Utilities|String|StringToName "DamagedPlayerRecently") true))

(event Game|Damage|EventAnyDamage
  (params (Damage :type Float%20%28single-precision%29) (DamageType :type Damage%20Type%20Object%20Reference) (InstigatedBy :type Controller%20Object%20Reference) (DamageCauser :type Actor%20Object%20Reference))
  (bind _capsulecomponent (Variables|Collision|GetCapsuleComponent))
  (Game|SpawnActorfromClass "/Game/FirstPerson/Blueprints/BP_PasswordNote.BP_PasswordNote_C" (Math|Transform|MakeTransform (Transformation|GetWorldLocation _capsulecomponent) (Transformation|GetWorldRotation _capsulecomponent)) "Undefined" "MultiplyWithRoot" 0 0)
  (Actor|DestroyActor))

(fn ConstructionScript)