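; Actor component that gives its owner a chance to drop a password note when destroyed.
; On BeginPlay it binds DropLoot to the owner's OnDestroyed event, which rolls a random integer against DropChance as a percentage.
; A successful roll spawns BP_PasswordNote at the destroyed actor's location and rotation, forcing unit scale so the owner's model scale does not resize the note.
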(event Custom|Drop%20Loot
  (params (DestroyedActor :type Actor%20Object%20Reference))
  (if (<= (Math|Random|RandomInteger 100) (Variables|Default|GetDrop%20chance))
    (Game|SpawnActorfromClass "/Game/FirstPerson/Blueprints/BP_PasswordNote.BP_PasswordNote_C" (Math|Transform|MakeTransform (Transformation|GetActorLocation DestroyedActor) (Transformation|GetActorRotation DestroyedActor)) "Undefined" "MultiplyWithRoot" 0 0)))

(event EventBeginPlay
  (Game|BindEventtoOnDestroyed (Components|GetOwner) (delegate Custom|Drop%20Loot)))